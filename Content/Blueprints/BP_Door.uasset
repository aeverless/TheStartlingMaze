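; Door actor that swings open by a configurable rotation offset from its starting rotation and plays open or locked sounds.
; BeginPlay caches the closed and open rotations, and events OnOpen and OnLocked only play their sounds.
; While Opened, which is not set here, Tick lerps rotation using a smoothstep-eased alpha.
; That alpha advances every tick over OpenDuration, even before the door opens.
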(event EventBeginPlay
  (bind _output_get (Variables|Default|SetDefaultRotation (Transformation|GetActorRotation)))
  (Variables|Default|SetOpenRotation (Math|Rotator|CombineRotators _output_get (Variables|Default|GetOpenRotationDelta))))

(event Collision|EventActorBeginOverlap
  (params (OtherActor :type Actor%20Object%20Reference)))

(event EventTick
  (params (DeltaSeconds :type Float%20%28single-precision%29))
  (bind _output_get (Variables|Default|SetOpenAlpha (+ (Variables|Default|GetOpenAlpha) (/ DeltaSeconds (Variables|Default|GetOpenDuration)))))
  (bind _value (CallFunction|Smoothstep _output_get))
  (if (and (Variables|Default|GetbOpened) (Utilities|Operators|NotEqual(!=) (Transformation|GetActorRotation) (Variables|Default|GetOpenRotation) 0.5))
    (Transformation|SetActorRotation (Math|Rotator|Lerp(Rotator) (Variables|Default|GetDefaultRotation) (Variables|Default|GetOpenRotation) _value true))
    (if (>= (Variables|Default|GetOpenAlpha) 1.0)
      (Variables|Default|SetOpenAlpha 0.0))))

(event EventOnLocked
  (Audio|PlaySoundatLocation "/Game/Audio/SW_DoorLocked.SW_DoorLocked" (Transformation|GetActorLocation) "0, 0, 0" 1.0 1.0 0.0 0 0 0 0))

(event EventOnOpen
  (Audio|PlaySoundatLocation "/Game/Audio/SW_DoorOpen.SW_DoorOpen" (Transformation|GetActorLocation) "0, 0, 0" 1.0 1.0 0.0 0 0 0 0))

(fn ConstructionScript)

(fn Smoothstep
  (params (X :type Float%20%28double-precision%29))
  (return (Math|Float|Clamp(Float) (- (* (Math|Float|Square X) 3.0) (* (Math|Float|Power X 3.0) 2.0)))))